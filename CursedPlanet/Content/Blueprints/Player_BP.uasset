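; Player pawn Blueprint that turns input into movement, camera look and a hold-to-hover action.
; Forward and right axes add movement input along directions built from control yaw only, keeping movement independent of camera pitch.
; Camera axes feed controller yaw and pitch.
; Pressing Hover activates the HoverThruster component and releasing it deactivates it.
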(event Input|ActionEvents|InputActionHover
  (params (Key :type Key%20Structure :default "None"))
  (:Pressed
    (Components|Activation|SetActive (Variables|Default|GetHoverThruster) true false))
  (:Released
    (Components|Activation|SetActive (Variables|Default|GetHoverThruster) false false)))

(event Input|AxisEvents|InputAxisCameraYaw
  (params (AxisValue :type Float%20%28single-precision%29))
  (Pawn|Input|AddControllerYawInput AxisValue))

(event Input|AxisEvents|InputAxisMoveForward
  (params (AxisValue :type Float%20%28single-precision%29))
  (Pawn|Input|AddMovementInput (Math|Vector|GetForwardVector (Math|Rotator|MakeRotator 0.0 0.0 (.Yaw (Math|Rotator|BreakRotator (Pawn|GetControlRotation :!class /Script/Engine.Pawn))))) AxisValue false))

(event Input|AxisEvents|InputAxisMoveRight
  (params (AxisValue :type Float%20%28single-precision%29))
  (Pawn|Input|AddMovementInput (Math|Vector|GetRightVector (Math|Rotator|MakeRotator 0.0 0.0 (.Yaw (Math|Rotator|BreakRotator (Pawn|GetControlRotation :!class /Script/Engine.Pawn))))) AxisValue false))

(event Input|AxisEvents|InputAxisCameraPitch
  (params (AxisValue :type Float%20%28single-precision%29))
  (Pawn|Input|AddControllerPitchInput AxisValue))

(fn ConstructionScript)